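; Interactable flower that rises when FlowerGoUp is called, up to a maximum height, with a configurable petal color set through a dynamic material.
; Each rise restarts a five-second timer whose decay check can let Tick lower the flower toward its target height.
; GetCaterpillared pulls it down toward its start height.
; A player collider overlapping its box starts a looping timer that sinks it according to the character's water level.
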(event `self.ReceiveBeginPlay`
  (bind _output_get (set `self.StartLocation` (`self.K2_GetActorLocation`)))
  (bind _x (.x _output_get))
  (bind _y (.y _output_get))
  (bind _z (.z _output_get))
  (set `self.TargetLocation` (`KismetMathLibrary.MakeVector` _x _y (+ _z (* (`self.MoveUpAmount`) 100.0))))
  (set `self.MaxLocation` (`KismetMathLibrary.MakeVector` _x _y (+ _z (* (`self.MaxUpAmount`) 100.0)))))

(event `self.ReceiveTick`
  (params (DeltaSeconds :type "Float (single-precision)"))
  (if (and (`self.Decaying`) (< (.z (`self.TargetLocation`)) (.z (`self.K2_GetActorLocation`))))
    (`self.K2_SetActorLocation` (`KismetMathLibrary.MakeVector` (.x (`self.K2_GetActorLocation`)) (.y (`self.K2_GetActorLocation`)) (+ (.z (`self.K2_GetActorLocation`)) -1.0)))
    (else
      (set `self.Decaying` false))))

(event `FlowerGoUp`
  (bind _flowerdecaytimer (`self.FlowerDecayTimer`))
  ; Savannah Nonsense - Couldn't call the above event from a different blueprint, so I made a new event. Mb, I know this is ugly.
  (set `self.Decaying` false)
  (if (`KismetSystemLibrary.K2_IsValidTimerHandle` _flowerdecaytimer)
    (`KismetSystemLibrary.K2_ClearAndInvalidateTimerHandle` _flowerdecaytimer))
  (bind _returnvalue (`KismetSystemLibrary.K2_SetTimerDelegate` (delegate `FlowerDecay`) 5.0))
  (set `self.FlowerDecayTimer` _returnvalue)
  (if (not (<= (.z (`self.MaxLocation`)) (.z (`self.K2_GetActorLocation`))))
    (`self.K2_SetActorLocation` (`KismetMathLibrary.MakeVector` (.x (`self.K2_GetActorLocation`)) (.y (`self.K2_GetActorLocation`)) (+ (.z (`self.K2_GetActorLocation`)) 1.0)))))

(event `FlowerDecay`
  (bind _returnvalue (`GameplayStatics.GetActorOfClass` "/Game/ThirdPerson/Blueprints/BP_ThirdPersonCharacter.BP_ThirdPersonCharacter_C"))
  (bind _output_get (set `self.Decaying` (and (not (and (`/Game/ThirdPerson/Blueprints/BP_ThirdPersonCharacter.WateringRN` _returnvalue) (`self.IsMoving`))) (< (.z (`self.TargetLocation`)) (.z (`self.K2_GetActorLocation`))))))
  (`KismetSystemLibrary.PrintString` (`KismetStringLibrary.Conv_BoolToString` _output_get)))

(event `GetCaterpillared`
  (if (< (.z (`self.StartLocation`)) (.z (`self.K2_GetActorLocation`)))
    (`self.K2_SetActorLocation` (`KismetMathLibrary.MakeVector` (.x (`self.K2_GetActorLocation`)) (.y (`self.K2_GetActorLocation`)) (+ (.z (`self.K2_GetActorLocation`)) -2.0)))))

(event `self.Box.OnComponentBeginOverlap`
  (params (OverlappedComponent :type "PrimitiveComponent Object Reference") (OtherActor :type "Actor Object Reference") (OtherComp :type "PrimitiveComponent Object Reference") (OtherBodyIndex :type Integer) (bFromSweep :type Boolean) (SweepResult :type "HitResult Structure (by ref)"))
  (`KismetSystemLibrary.PrintString` "Overlapped?")
  (bind _output_get (set `self.IsWeighedDown` (>= (`KismetArrayLibrary.Array_Find` (`ActorComponent.ComponentTags` OtherComp) "PlayerCollider") 0)))
  (if _output_get
    (`KismetSystemLibrary.PrintString` "Okay True")
    (bind _returnvalue (`KismetSystemLibrary.K2_SetTimerDelegate` (delegate `WeighDownFlower`) 0.01 true))))

(event `WeighDownFlower`
  (`KismetSystemLibrary.PrintString` "You're in weigh down flower")
  (if (`self.IsWeighedDown`)
    (bind _returnvalue (`GameplayStatics.GetActorOfClass` "/Game/ThirdPerson/Blueprints/BP_ThirdPersonCharacter.BP_ThirdPersonCharacter_C"))
    (`self.K2_SetActorLocation` (`KismetMathLibrary.MakeVector` (.x (`self.K2_GetActorLocation`)) (.y (`self.K2_GetActorLocation`)) (- (.z (`self.K2_GetActorLocation`)) (* (`/Game/ThirdPerson/Blueprints/BP_ThirdPersonCharacter.WaterLevelPercent` _returnvalue) 0.5))))))

(event `self.Box.OnComponentEndOverlap`
  (params (OverlappedComponent :type "PrimitiveComponent Object Reference") (OtherActor :type "Actor Object Reference") (OtherComp :type "PrimitiveComponent Object Reference") (OtherBodyIndex :type Integer))
  (cast `/Game/ThirdPerson/Blueprints/BP_ThirdPersonCharacter` OtherActor)
  (set `self.IsWeighedDown` false)
  (`KismetSystemLibrary.K2_ClearAndInvalidateTimerHandle` (stale `self.Box.OnComponentBeginOverlap` _returnvalue)))

(fn `UserConstructionScript`
  (bind _returnvalue (`PrimitiveComponent.CreateDynamicMaterialInstance` (`self.cylinder`) 0 "/Game/LevelPrototyping/Meshes/dynamic_petal_color.dynamic_petal_color" "None"))
  (bind _output_get (set `self.PetalMID` _returnvalue))
  (`MaterialInstanceDynamic.SetVectorParameterValue` _output_get "PetalColor" (`self.PetalColor`)))