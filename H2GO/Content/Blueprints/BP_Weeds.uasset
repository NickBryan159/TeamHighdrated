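; BP_Weeds is a hazard actor that slows the player to a quarter of walk speed while inside its sphere.
; Sphere overlap events filter for components tagged PlayerCollider and cast the other actor to BP_ThirdPersonCharacter.
; Entering divides MaxWalkSpeed and leaving multiplies it back, each copying the result into the character's BaseSpeed.
; The change is relative to current speed, so overlapping patches compound.
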(event `self.ReceiveActorBeginOverlap`
  (params (OtherActor :type "Actor Object Reference")))

(event `self.ReceiveActorEndOverlap`
  (params (OtherActor :type "Actor Object Reference")))

(event `self.Sphere.OnComponentBeginOverlap`
  (params (OverlappedComponent :type "PrimitiveComponent Object Reference") (OtherActor :type "Actor Object Reference") (OtherComp :type "PrimitiveComponent Object Reference") (OtherBodyIndex :type Integer) (bFromSweep :type Boolean) (SweepResult :type "HitResult Structure (by ref)"))
  (if (>= (`KismetArrayLibrary.Array_Find` (`ActorComponent.ComponentTags` OtherComp) "PlayerCollider") 0)
    (bind _asbp_third_person_character (cast `/Game/ThirdPerson/Blueprints/BP_ThirdPersonCharacter` OtherActor))
    (bind _charactermovement (`Character.CharacterMovement` _asbp_third_person_character))
    (bind _output_get (set `CharacterMovementComponent.MaxWalkSpeed` (/ (`CharacterMovementComponent.MaxWalkSpeed` _charactermovement) 4.0) _charactermovement))
    (set `/Game/ThirdPerson/Blueprints/BP_ThirdPersonCharacter.BaseSpeed` _output_get _asbp_third_person_character)))

(event `self.Sphere.OnComponentEndOverlap`
  (params (OverlappedComponent :type "PrimitiveComponent Object Reference") (OtherActor :type "Actor Object Reference") (OtherComp :type "PrimitiveComponent Object Reference") (OtherBodyIndex :type Integer))
  (if (>= (`KismetArrayLibrary.Array_Find` (`ActorComponent.ComponentTags` OtherComp) "PlayerCollider") 0)
    (bind _asbp_third_person_character (cast `/Game/ThirdPerson/Blueprints/BP_ThirdPersonCharacter` OtherActor))
    (bind _charactermovement (`Character.CharacterMovement` _asbp_third_person_character))
    (bind _output_get (set `CharacterMovementComponent.MaxWalkSpeed` (* (`CharacterMovementComponent.MaxWalkSpeed` _charactermovement) 4.0) _charactermovement))
    (set `/Game/ThirdPerson/Blueprints/BP_ThirdPersonCharacter.BaseSpeed` _output_get _asbp_third_person_character)))

(fn `UserConstructionScript`)