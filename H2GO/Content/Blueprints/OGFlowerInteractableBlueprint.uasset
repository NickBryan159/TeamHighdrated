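; Interactable flower actor that rises toward a height offset while watered and sinks back once left alone.
; Another Blueprint calls FlowerGoUp, which nudges it up per call, cancels decay and restarts a delay timer.
; When the timer fires, FlowerDecay checks the character's watering state and may set Decaying, letting Tick step it down to its start.
; A separate hold-interact event lifts it via a timeline lerp.
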(event `self.InteractHoldStart`
  (`KismetSystemLibrary.PrintString` "Interacted!")
  (bind _output_get (set `self.StartLocation` (`self.K2_GetActorLocation`)))
  (set `self.TargetLocation` (+ _output_get (`KismetMathLibrary.MakeVector` 0.0 0.0 (`KismetMathLibrary.Conv_IntToDouble` (`self.MoveUpAmount`)))))
  (bind (_direction _alpha) (`Timeline|MoveUp` :!via `PlayFromStart`)
    (:`Update`
      (`self.K2_SetActorLocation` (`KismetMathLibrary.VLerp` (`self.StartLocation`) (`self.TargetLocation`) _alpha)))))

(event `self.ReceiveBeginPlay`
  (bind _output_get (set `self.StartLocation` (`self.K2_GetActorLocation`)))
  (set `self.TargetLocation` (`KismetMathLibrary.MakeVector` (.x _output_get) (.y _output_get) (+ (.z _output_get) (`self.MoveUpAmount`)))))

(event `self.ReceiveTick`
  (params (DeltaSeconds :type "Float (single-precision)"))
  (if (and (`self.Decaying`) (< (.z (`self.StartLocation`)) (.z (`self.K2_GetActorLocation`))))
    (`self.K2_SetActorLocation` (`KismetMathLibrary.MakeVector` (.x (`self.K2_GetActorLocation`)) (.y (`self.K2_GetActorLocation`)) (+ (.z (`self.K2_GetActorLocation`)) -1.0)))))

(event `FlowerGoUp`
  (bind _flowerdecaytimer (`self.FlowerDecayTimer`))
  ; Savannah Nonsense - Couldn't call the above event from a different blueprint, so I made a new event. Mb, I know this is ugly.
  (set `self.Decaying` false)
  (if (`KismetSystemLibrary.K2_IsValidTimerHandle` _flowerdecaytimer)
    (`KismetSystemLibrary.K2_ClearAndInvalidateTimerHandle` _flowerdecaytimer))
  (bind _returnvalue (`KismetSystemLibrary.K2_SetTimerDelegate` (delegate `FlowerDecay`) 5.0))
  (set `self.FlowerDecayTimer` _returnvalue)
  (if (not (<= (.z (`self.TargetLocation`)) (.z (`self.K2_GetActorLocation`))))
    (`self.K2_SetActorLocation` (`KismetMathLibrary.MakeVector` (.x (`self.K2_GetActorLocation`)) (.y (`self.K2_GetActorLocation`)) (+ (.z (`self.K2_GetActorLocation`)) 1.0)))
    (set `self.LastWatered` 0.0)))

(event `FlowerDecay`
  (`KismetSystemLibrary.PrintString` "Creepah")
  (bind _returnvalue (`GameplayStatics.GetActorOfClass` "/Game/ThirdPerson/Blueprints/BP_ThirdPersonCharacter.BP_ThirdPersonCharacter_C"))
  (set `self.Decaying` (and (not (and (`/Game/ThirdPerson/Blueprints/BP_ThirdPersonCharacter.WateringRN` _returnvalue) (`self.IsMoving`))) (< (.z (`self.StartLocation`)) (.z (`self.K2_GetActorLocation`))))))

(fn `UserConstructionScript`
  (bind _output_get (set `self.StartLocation` (`self.K2_GetActorLocation`)))
  (set `self.TargetLocation` (`KismetMathLibrary.MakeVector` (.x _output_get) (.y _output_get) (+ (.z _output_get) (`self.MoveUpAmount`)))))