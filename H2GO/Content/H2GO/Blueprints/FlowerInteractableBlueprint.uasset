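; Interactable flower actor that rises vertically by MoveUpAmount when triggered.
; InteractHoldStart records the current location, offsets it on Z, and plays the MoveUp timeline to lerp the actor to that target.
; FlowerGoUp duplicates this logic on its own timeline as a workaround so other Blueprints can trigger the rise, per the author's note.
; Both events print a debug string and share the start and target location variables.
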(event `self.InteractHoldStart`
  (`KismetSystemLibrary.PrintString` "Interacted!")
  (bind _output_get (set `self.StartLocation` (`self.K2_GetActorLocation`)))
  (set `self.TargetLocation` (+ _output_get (`KismetMathLibrary.MakeVector` 0.0 0.0 (`KismetMathLibrary.Conv_IntToDouble` (`self.MoveUpAmount`)))))
  (bind (_direction _alpha) (`Timeline|MoveUp` :!via `PlayFromStart`)
    (:`Update`
      (`self.K2_SetActorLocation` (`KismetMathLibrary.VLerp` (`self.StartLocation`) (`self.TargetLocation`) _alpha)))))

(event `FlowerGoUp`
  ; Savannah Nonsense - Couldn't call the above event from a different blueprint, so I made a new event. Mb, I know this is ugly.
  (`KismetSystemLibrary.PrintString` "Interacted!")
  (bind _output_get (set `self.StartLocation` (`self.K2_GetActorLocation`)))
  (set `self.TargetLocation` (+ _output_get (`KismetMathLibrary.MakeVector` 0.0 0.0 (`KismetMathLibrary.Conv_IntToDouble` (`self.MoveUpAmount`)))))
  (bind (_direction _alpha) (`Timeline|Timeline` :!via `PlayFromStart`)
    (:`Update`
      (`self.K2_SetActorLocation` (`KismetMathLibrary.VLerp` (`self.StartLocation`) (`self.TargetLocation`) _alpha)))))

(fn `UserConstructionScript`)